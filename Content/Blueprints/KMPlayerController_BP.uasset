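; KMPlayerController_BP is a player controller that switches the player between the sign-in screen and the main menu.
; BeginPlay creates the sign-in widget and adds it to the viewport.
; The Singedin event hides that widget, then creates and shows a new main menu widget on each call.
; OpenSigninScreen shows the existing sign-in widget again and hides the main menu.
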(event `self.ReceiveBeginPlay`
  (bind _returnvalue (`|CreateWidget` "/Game/HUD/SigInWidget.SigInWidget_C" null self))
  (bind _output_get (set `self.SingInWidget` _returnvalue))
  (`UserWidget.AddToViewport` _output_get 0))

(event `self.SingedIn`
  (`Widget.SetVisibility` (`self.SingInWidget`) "Hidden")
  ;[1 1 1] Create MainMeny
  (bind _returnvalue (`|CreateWidget` "/Game/HUD/MainMenuWidget.MainMenuWidget_C" null self))
  (bind _output_get (set `self.MainMenuWidget` _returnvalue))
  (`UserWidget.AddToViewport` _output_get 0)
  (`KismetSystemLibrary.PrintString` "Created mainMne"))

(event `self.OpenSignInScreen`
  (`Widget.SetVisibility` (`self.SingInWidget`) "Visible")
  (`Widget.SetVisibility` (`self.MainMenuWidget`) "Hidden"))

(fn `UserConstructionScript`)