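; MainGameActor is an actor that manages the switch between the sign-in screen and the main menu.
; On BeginPlay it shows the mouse cursor, creates both widgets and adds them to the viewport, with the main menu hidden.
; SignedIn and SignOut toggle the visibility of the two widgets, so neither is recreated when switching.
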(event `self.ReceiveBeginPlay`
  (set `PlayerController.bShowMouseCursor` true (`GameplayStatics.GetPlayerController` 0))
  ;[1 1 1] Create SignInWidget
  (bind _returnvalue (`|CreateWidget` "/Game/Blueprints/SignIn_BP.SignIn_BP_C" null self))
  (bind _output_get (set `self.SignInWidget` _returnvalue))
  (`UserWidget.AddToViewport` _output_get 0)
  (bind _returnvalue_2 (`|CreateWidget` "/Game/Blueprints/MainMenu.MainMenu_C" null self))
  (bind _output_get_2 (set `self.MainMenuWidget` _returnvalue_2))
  (`UserWidget.AddToViewport` _output_get_2 0)
  (`Widget.SetVisibility` _output_get_2 "Hidden"))

(fn `SignedIn`
  (`KismetSystemLibrary.PrintString` "MainActor opened mainmenu")
  (`Widget.SetVisibility` (`self.SignInWidget`) "Hidden")
  (`Widget.SetVisibility` (`self.MainMenuWidget`) "Visible"))

(fn `SignOut`
  (`Widget.SetVisibility` (`self.SignInWidget`) "Visible")
  (`Widget.SetVisibility` (`self.MainMenuWidget`) "Hidden"))

(fn `UserConstructionScript`)